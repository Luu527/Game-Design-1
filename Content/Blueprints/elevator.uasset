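; Elevator actor with a sliding part, likely its door, and trigger components that react only to BP_ThirdPersonCharacterCustom.
; Entering trigger R plays an electronic door-opening sound at the root and shifts component E along X, while leaving R shifts it back.
; Entering trigger W sets the root component to a fixed location, relocating the whole actor with no return logic.
; All moves are instant, unswept location sets without interpolation.
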(event `self.r.OnComponentBeginOverlap`
  (params (OverlappedComponent :type "PrimitiveComponent Object Reference") (OtherActor :type "Actor Object Reference") (OtherComp :type "PrimitiveComponent Object Reference") (OtherBodyIndex :type Integer) (bFromSweep :type Boolean) (SweepResult :type "HitResult Structure (by ref)"))
  (cast `/Game/Blueprints/BP_ThirdPersonCharacterCustom` OtherActor)
  (`GameplayStatics.PlaySoundAtLocation` "/Game/Audio/electronic-door-opening-102496.electronic-door-opening-102496" (`SceneComponent.K2_GetComponentLocation` (`self.DefaultSceneRoot`)) (struct) 1.0 1.0 0.0 null null null null)
  (`SceneComponent.K2_SetRelativeLocation` (`self.e`) (15.0 0.0 0.0) false false))

(event `self.r.OnComponentEndOverlap`
  (params (OverlappedComponent :type "PrimitiveComponent Object Reference") (OtherActor :type "Actor Object Reference") (OtherComp :type "PrimitiveComponent Object Reference") (OtherBodyIndex :type Integer))
  (cast `/Game/Blueprints/BP_ThirdPersonCharacterCustom` OtherActor)
  (`SceneComponent.K2_SetRelativeLocation` (`self.e`) (-175.0 0.0 0.0) false false))

(event `self.w.OnComponentBeginOverlap`
  (params (OverlappedComponent :type "PrimitiveComponent Object Reference") (OtherActor :type "Actor Object Reference") (OtherComp :type "PrimitiveComponent Object Reference") (OtherBodyIndex :type Integer) (bFromSweep :type Boolean) (SweepResult :type "HitResult Structure (by ref)"))
  (cast `/Game/Blueprints/BP_ThirdPersonCharacterCustom` OtherActor)
  (`SceneComponent.K2_SetRelativeLocation` (`self.DefaultSceneRoot`) (0.0 150.0 0.0) false false))

(fn `UserConstructionScript`)