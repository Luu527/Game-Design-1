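; BP_AccessCard is a pickup that grants the player character an access card key.
; When BP_ThirdPersonCharacterCustom overlaps the GetCard component, it sets HasKey on the character and its own BIsKeyPickUp flag.
; It then shows the W_GetAccessCard widget, plays a pickup sound using the Card's world scale as the location, and removes the widget and itself after a short delay.
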(event `self.GetCard.OnComponentBeginOverlap`
  (params (OverlappedComponent :type "PrimitiveComponent Object Reference") (OtherActor :type "Actor Object Reference") (OtherComp :type "PrimitiveComponent Object Reference") (OtherBodyIndex :type Integer) (bFromSweep :type Boolean) (SweepResult :type "HitResult Structure (by ref)"))
  (bind _asbp_third_person_character_custom (cast `/Game/Blueprints/BP_ThirdPersonCharacterCustom` OtherActor))
  (set `/Game/Blueprints/BP_ThirdPersonCharacterCustom.HasKey` true _asbp_third_person_character_custom)
  (set `self.BIsKeyPickUp` true)
  (bind _returnvalue (`|CreateWidget` "/Game/Widgets/W_GetAccessCard.W_GetAccessCard_C"))
  (`UserWidget.AddToViewport` _returnvalue 0)
  (`GameplayStatics.PlaySoundAtLocation` "/Game/Audio/pick-up-sfx-38516.pick-up-sfx-38516" (`SceneComponent.K2_GetComponentScale` (`self.Card`)) (struct) 1.0 1.0 0.0 null null null null)
  (`KismetSystemLibrary.Delay` 0.5)
  (`Widget.RemoveFromParent` _returnvalue)
  (`self.K2_DestroyActor`))

(fn `UserConstructionScript`)