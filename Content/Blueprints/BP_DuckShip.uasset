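; BP_DuckShip is a duck ship actor that reacts when the player character comes near without a ship key.
; On sphere overlap by BP_ThirdPersonCharacterCustom, if ShipKey is not above zero, it plays a quack at the Duck component and shows a newly created W_Level2Ship widget.
; When the character leaves the sphere, it removes that widget from the screen.
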(event `self.Sphere.OnComponentBeginOverlap`
  (params (OverlappedComponent :type "PrimitiveComponent Object Reference") (OtherActor :type "Actor Object Reference") (OtherComp :type "PrimitiveComponent Object Reference") (OtherBodyIndex :type Integer) (bFromSweep :type Boolean) (SweepResult :type "HitResult Structure (by ref)"))
  (cast `/Game/Blueprints/BP_ThirdPersonCharacterCustom` OtherActor)
  (if (not (> (`self.ShipKey`) 0))
    (`GameplayStatics.PlaySoundAtLocation` "/Game/Audio/duck-quack-40345.duck-quack-40345" (`SceneComponent.K2_GetComponentLocation` (`self.duck`)) (struct) 1.0 1.0 0.0 null null null null)
    (bind _returnvalue (`|CreateWidget` "/Game/Widgets/W_Level2Ship.W_Level2Ship_C"))
    (`UserWidget.AddToViewport` _returnvalue 0)))

(event `self.Sphere.OnComponentEndOverlap`
  (params (OverlappedComponent :type "PrimitiveComponent Object Reference") (OtherActor :type "Actor Object Reference") (OtherComp :type "PrimitiveComponent Object Reference") (OtherBodyIndex :type Integer))
  (cast `/Game/Blueprints/BP_ThirdPersonCharacterCustom` OtherActor)
  (`Widget.RemoveFromParent` (stale `self.Sphere.OnComponentBeginOverlap` _returnvalue)))

(fn `UserConstructionScript`)