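; BP_weapoon1 is a weapon pickup actor that the player collects by pressing E while near it.
; Its Box overlap with BP_ThirdPersonCharacterCustom toggles the actor's input for player 0 and shows or removes the W_pickUpWeapon prompt.
; PressE removes the prompt, plays a click sound, shows the W_pickUpWeaponExplian widget and destroys the actor.
; The graph itself grants no weapon to the character.
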(event `self.Box.OnComponentBeginOverlap`
  (params (OverlappedComponent :type "PrimitiveComponent Object Reference") (OtherActor :type "Actor Object Reference") (OtherComp :type "PrimitiveComponent Object Reference") (OtherBodyIndex :type Integer) (bFromSweep :type Boolean) (SweepResult :type "HitResult Structure (by ref)"))
  (cast `/Game/Blueprints/BP_ThirdPersonCharacterCustom` OtherActor)
  (`self.EnableInput` (`GameplayStatics.GetPlayerController` 0))
  (bind _returnvalue (`|CreateWidget` "/Game/Widgets/W_pickUpWeapon.W_pickUpWeapon_C"))
  (`UserWidget.AddToViewport` _returnvalue 0))

(event `self.Box.OnComponentEndOverlap`
  (params (OverlappedComponent :type "PrimitiveComponent Object Reference") (OtherActor :type "Actor Object Reference") (OtherComp :type "PrimitiveComponent Object Reference") (OtherBodyIndex :type Integer))
  (cast `/Game/Blueprints/BP_ThirdPersonCharacterCustom` OtherActor)
  (`self.DisableInput` (`GameplayStatics.GetPlayerController` 0))
  (`Widget.RemoveFromParent` (stale `self.Box.OnComponentBeginOverlap` _returnvalue)))

(event `InputAction|PressE`
  (params (Key :type "Key Structure"))
  (:`Pressed`
    (`Widget.RemoveFromParent` (stale `self.Box.OnComponentBeginOverlap` _returnvalue))
    (`GameplayStatics.SpawnSoundAtLocation` "/Game/Audio/old-radio-button-click-97549.old-radio-button-click-97549" (`SceneComponent.K2_GetComponentLocation` (`self.Box`)) (struct) 1.0 1.0 0.0 null null)
    (bind _returnvalue (`|CreateWidget` "/Game/Widgets/W_pickUpWeaponExplian.W_pickUpWeaponExplian_C"))
    (`UserWidget.AddToViewport` _returnvalue 0)
    (`self.K2_DestroyActor`)))

(fn `UserConstructionScript`)