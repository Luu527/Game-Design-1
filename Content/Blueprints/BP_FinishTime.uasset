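; BP_FinishTime is a finish-line trigger that times and displays the player's laps.
; On BeginPlay it adds the W_FinishTimeline widget to the viewport and starts a self-calling 0.1-second Delay loop.
; That loop prints and writes the current lap time to the widget, measured as real time since LastTimestamp.
; When BP_ThirdPersonCharacterCustom overlaps the Box, it prints that lap's time and resets LastTimestamp.
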(event `self.ReceiveBeginPlay`
  (bind _returnvalue (`|CreateWidget` "/Game/Widgets/W_FinishTimeline.W_FinishTimeline_C"))
  (bind _output_get (set `self.W_TimerWidget` _returnvalue))
  (`UserWidget.AddToViewport` _output_get 0)
  (`self.On screen timer`))

(event `On screen timer`
  (bind _returnvalue (`KismetStringLibrary.Concat_StrStr` "Current Lap " (`KismetTextLibrary.Conv_TextToString` (`KismetTextLibrary.Conv_DoubleToText` (- (`GameplayStatics.GetRealTimeSeconds`) (`self.Last Timestamp`)) "HalfToEven" false true 1 324 0 1)) "seconds"))
  ;[1 1 1] On screen timer
  (`KismetSystemLibrary.PrintString` _returnvalue true true (struct :`G` 0.66 :`B` 1.0 :`A` 1.0) 0.1)
  (set `TextBlock.Text` (`KismetTextLibrary.Conv_StringToText` _returnvalue) (`/Game/Widgets/W_FinishTimeline.currentTimeText` (`self.W_TimerWidget`))) ; set text
  (`KismetSystemLibrary.Delay` 0.1)
  (`self.On screen timer`))

(event `self.Box.OnComponentBeginOverlap`
  (params (OverlappedComponent :type "PrimitiveComponent Object Reference") (OtherActor :type "Actor Object Reference") (OtherComp :type "PrimitiveComponent Object Reference") (OtherBodyIndex :type Integer) (bFromSweep :type Boolean) (SweepResult :type "HitResult Structure (by ref)"))
  (cast `/Game/Blueprints/BP_ThirdPersonCharacterCustom` OtherActor)
  (`KismetSystemLibrary.PrintString` (`KismetStringLibrary.Concat_StrStr` "that lap took " (`KismetTextLibrary.Conv_TextToString` (`KismetTextLibrary.Conv_DoubleToText` (- (`GameplayStatics.GetRealTimeSeconds`) (`self.Last Timestamp`)) "HalfToEven" false true 1 324 0 1)) " seconds!"))
  (set `self.Last Timestamp` (`GameplayStatics.GetRealTimeSeconds`)))

(fn `UserConstructionScript`)