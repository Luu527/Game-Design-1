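; Locked door actor that disappears when the player character walks into its Box trigger carrying at least one key.
; Begin overlap casts to BP_ThirdPersonCharacterCustom and checks KeyCount, destroying the actor without decrementing the count.
; With no key, it creates a W_Level1 widget, stores it as DoorLock and adds it to the viewport.
; End overlap removes that widget behind a negated IsValid check that has no visible input.
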(event `self.Box.OnComponentBeginOverlap`
  (params (OverlappedComponent :type "PrimitiveComponent Object Reference") (OtherActor :type "Actor Object Reference") (OtherComp :type "PrimitiveComponent Object Reference") (OtherBodyIndex :type Integer) (bFromSweep :type Boolean) (SweepResult :type "HitResult Structure (by ref)"))
  (bind _asbp_third_person_character_custom (cast `/Game/Blueprints/BP_ThirdPersonCharacterCustom` OtherActor))
  (if (> (`/Game/Blueprints/BP_ThirdPersonCharacterCustom.Key Count` _asbp_third_person_character_custom) 0)
    (`self.K2_DestroyActor`)
    (else
      (bind _returnvalue (`|CreateWidget` "/Game/Widgets/W_Level1.W_Level1_C" (`GameplayStatics.GetPlayerController` 0)))
      (bind _output_get (set `self.DoorLock` _returnvalue))
      (`UserWidget.AddToViewport` _output_get 10))))

(event `self.Box.OnComponentEndOverlap`
  (params (OverlappedComponent :type "PrimitiveComponent Object Reference") (OtherActor :type "Actor Object Reference") (OtherComp :type "PrimitiveComponent Object Reference") (OtherBodyIndex :type Integer))
  (cast `/Game/Blueprints/BP_ThirdPersonCharacterCustom` OtherActor)
  (`/Engine/EditorBlueprintResources/StandardMacros.IsValid` null
    (:`Is Not Valid`
      (`Widget.RemoveFromParent` (`self.DoorLock`)))))

(fn `UserConstructionScript`)