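; Control room door that slides vertically for a player character holding a key and refuses entry otherwise.
; Entering the box trigger with the key plays an opening sound and runs a timeline that drives the door's relative location.
; Without the key, it plays an error sound and shows the Level 2 control room door widget.
; Leaving removes the widget and, for key holders, reverses the timeline from its end to close the door.
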(event `self.Box.OnComponentBeginOverlap`
  (params (OverlappedComponent :type "PrimitiveComponent Object Reference") (OtherActor :type "Actor Object Reference") (OtherComp :type "PrimitiveComponent Object Reference") (OtherBodyIndex :type Integer) (bFromSweep :type Boolean) (SweepResult :type "HitResult Structure (by ref)"))
  (bind _asbp_third_person_character_custom (cast `/Game/Blueprints/BP_ThirdPersonCharacterCustom` OtherActor))
  (if (`/Game/Blueprints/BP_ThirdPersonCharacterCustom.HasKey` _asbp_third_person_character_custom)
    (`GameplayStatics.PlaySoundAtLocation` "/Game/Audio/sfx-door-open-85017.sfx-door-open-85017" (`SceneComponent.GetSocketLocation` (`self.door`) "None") (struct) 1.0 1.0 0.0 null null null null)
    (bind (_direction _newtrack_1) (`Timeline|Timeline` :!label _label)
      (:`Update`
        (`SceneComponent.K2_SetRelativeLocation` (`self.door`) (* _newtrack_1 (0.0 0.0 600.0)) false false)))
    (else
      (`GameplayStatics.PlaySoundAtLocation` "/Game/Audio/wrong-47985.wrong-47985" (`SceneComponent.K2_GetComponentLocation` (`self.door`)) (struct) 1.0 1.0 0.0 null null null null)
      (bind _returnvalue (`|CreateWidget` "/Game/Widgets/W_Level2ControlroomDoor.W_Level2ControlroomDoor_C" (`GameplayStatics.GetPlayerController` 0)))
      (`UserWidget.AddToViewport` _returnvalue 10))))

(event `self.Box.OnComponentEndOverlap`
  (params (OverlappedComponent :type "PrimitiveComponent Object Reference") (OtherActor :type "Actor Object Reference") (OtherComp :type "PrimitiveComponent Object Reference") (OtherBodyIndex :type Integer))
  (bind _asbp_third_person_character_custom (cast `/Game/Blueprints/BP_ThirdPersonCharacterCustom` OtherActor))
  (`Widget.RemoveFromParent` (stale `self.Box.OnComponentBeginOverlap` _returnvalue))
  (if (`/Game/Blueprints/BP_ThirdPersonCharacterCustom.HasKey` _asbp_third_person_character_custom)
    (goto _label :!via `ReverseFromEnd`)))

(fn `UserConstructionScript`)